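; Configurable space skybox Blueprint that drives the look of its SpaceCubemap component through exposed variables.
; The construction script creates a dynamic instance of M_Space_CubemapInst1 on that component and copies every variable into the matching material parameter.
; Parameters cover two star layers and five texture layers with placement, rotation, density and color grading, plus overall emissive and opacity.
; BeginPlay and Tick are empty, so nothing updates at runtime.
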(event `self.ReceiveBeginPlay`)

(event `self.ReceiveTick`
  (params (DeltaSeconds :type "Float (single-precision)")))

(fn `UserConstructionScript`
  (bind _material_instance (`self.Material_Instance`))
  (bind _returnvalue (`PrimitiveComponent.CreateDynamicMaterialInstance` (`self.Space_Cubemap`) 0 "/Game/Space_Skybox/Material/M_Space_CubemapInst1.M_Space_CubemapInst1" "None"))
  (set `self.Material_Instance` _returnvalue)
  (`MaterialInstanceDynamic.SetTextureParameterValue` _returnvalue "Tex_Stars_1" (`self.Tex_Stars_1`))
  (`MaterialInstanceDynamic.SetTextureParameterValue` _material_instance "Tex_Stars_1" (`self.Tex_Stars_1`))
  (`MaterialInstanceDynamic.SetScalarParameterValue` _material_instance "Stars1_Power" (`self.Stars1_Power`))
  (`MaterialInstanceDynamic.SetScalarParameterValue` _returnvalue "Stars1_Power" (`self.Stars1_Power`))
  (`MaterialInstanceDynamic.SetScalarParameterValue` _material_instance "Stars1_Desaturation" (`self.Stars1_Desaturation`))
  (`MaterialInstanceDynamic.SetScalarParameterValue` _returnvalue "Stars1_Desaturation" (`self.Stars1_Desaturation`))
  (`MaterialInstanceDynamic.SetVectorParameterValue` _returnvalue "Stars1_Color" (`self.Stars1_Color`))
  (`MaterialInstanceDynamic.SetVectorParameterValue` _material_instance "Stars1_Color" (`self.Stars1_Color`))
  (`MaterialInstanceDynamic.SetTextureParameterValue` _returnvalue "Tex_Stars_2" (`self.Tex_Stars_2`))
  (`MaterialInstanceDynamic.SetTextureParameterValue` _material_instance "Tex_Stars_2" (`self.Tex_Stars_2`))
  (`MaterialInstanceDynamic.SetScalarParameterValue` _material_instance "Stars2_Power" (`self.Stars2_Power`))
  (`MaterialInstanceDynamic.SetScalarParameterValue` _returnvalue "Stars2_Power" (`self.Stars2_Power`))
  (`MaterialInstanceDynamic.SetScalarParameterValue` _material_instance "Stars2_Desaturation" (`self.Stars2_Desaturation`))
  (`MaterialInstanceDynamic.SetScalarParameterValue` _returnvalue "Stars2_Desaturation" (`self.Stars2_Desaturation`))
  (`MaterialInstanceDynamic.SetVectorParameterValue` _returnvalue "Stars2_Color" (`self.Stars2_Color`))
  (`MaterialInstanceDynamic.SetVectorParameterValue` _material_instance "Stars2_Color" (`self.Stars2_Color`))
  (`MaterialInstanceDynamic.SetTextureParameterValue` _returnvalue "Tex1_Color" (`self.Tex1_Color`))
  (`MaterialInstanceDynamic.SetTextureParameterValue` _material_instance "Tex1_Color" (`self.Tex1_Color`))
  (`MaterialInstanceDynamic.SetVectorParameterValue` _returnvalue "Tex1_Scale" (`self.Tex1_Scale`))
  (`MaterialInstanceDynamic.SetScalarParameterValue` _returnvalue "Tex1_Radius" (`self.Tex1_Radius`))
  (`MaterialInstanceDynamic.SetScalarParameterValue` _returnvalue "Tex1_Density" (`self.Tex1_Density`))
  (`MaterialInstanceDynamic.SetScalarParameterValue` _material_instance "Tex1_Density" (`self.Tex1_Density`))
  (`MaterialInstanceDynamic.SetScalarParameterValue` _returnvalue "Tex1_RotateAngle Z" (`self.Tex1_RotateAngle Z`))
  (`MaterialInstanceDynamic.SetScalarParameterValue` _material_instance "Tex1_RotateAngle Z" (`self.Tex1_RotateAngle Z`))
  (`MaterialInstanceDynamic.SetScalarParameterValue` _returnvalue "Tex1_RotateAngle Y" (`self.Tex1_RotateAngle Y`))
  (`MaterialInstanceDynamic.SetScalarParameterValue` _material_instance "Tex1_RotateAngle Y" (`self.Tex1_RotateAngle Y`))
  (`MaterialInstanceDynamic.SetScalarParameterValue` _returnvalue "Tex1_Red_Level" (`self.Tex1_Red_Level`))
  (`MaterialInstanceDynamic.SetScalarParameterValue` _material_instance "Tex1_Red_Level" (`self.Tex1_Red_Level`))
  (`MaterialInstanceDynamic.SetScalarParameterValue` _returnvalue "Tex1_Green_Level" (`self.Tex1_Green_Level`))
  (`MaterialInstanceDynamic.SetScalarParameterValue` _material_instance "Tex1_Green_Level" (`self.Tex1_Green_Level`))
  (`MaterialInstanceDynamic.SetScalarParameterValue` _returnvalue "Tex1_Blue_Level" (`self.Tex1_Blue_Level`))
  (`MaterialInstanceDynamic.SetScalarParameterValue` _material_instance "Tex1_Blue_Level" (`self.Tex1_Blue_Level`))
  (`MaterialInstanceDynamic.SetScalarParameterValue` _returnvalue "Tex1_Power" (`self.Tex1_Power`))
  (`MaterialInstanceDynamic.SetScalarParameterValue` _material_instance "Tex1_Power" (`self.Tex1_Power`))
  (`MaterialInstanceDynamic.SetScalarParameterValue` _returnvalue "Tex1_Saturation" (`self.Tex1_Saturation`))
  (`MaterialInstanceDynamic.SetScalarParameterValue` _material_instance "Tex1_Saturation" (`self.Tex1_Saturation`))
  (`MaterialInstanceDynamic.SetScalarParameterValue` _returnvalue "Tex1_Tone" (`self.Tex1_Tone`))
  (`MaterialInstanceDynamic.SetScalarParameterValue` _material_instance "Tex1_Tone" (`self.Tex1_Tone`))
  (`MaterialInstanceDynamic.SetTextureParameterValue` _returnvalue "Tex2_Color" (`self.Tex2_Color`))
  (`MaterialInstanceDynamic.SetTextureParameterValue` _material_instance "Tex2_Color" (`self.Tex2_Color`))
  (`MaterialInstanceDynamic.SetVectorParameterValue` _returnvalue "Tex2_Scale" (`self.Tex2_Scale`))
  (`MaterialInstanceDynamic.SetVectorParameterValue` _material_instance "Tex2_Scale" (`self.Tex2_Scale`))
  (`MaterialInstanceDynamic.SetScalarParameterValue` _returnvalue "Tex2_Radius" (`self.Tex2_Radius`))
  (`MaterialInstanceDynamic.SetScalarParameterValue` _material_instance "Tex2_Radius" (`self.Tex2_Radius`))
  (`MaterialInstanceDynamic.SetScalarParameterValue` _returnvalue "Tex2_Density" (`self.Tex2_Density`))
  (`MaterialInstanceDynamic.SetScalarParameterValue` _material_instance "Tex2_Density" (`self.Tex2_Density`))
  (`MaterialInstanceDynamic.SetScalarParameterValue` _returnvalue "Tex2_RotateAngle Z" (`self.Tex2_RotateAngle Z`))
  (`MaterialInstanceDynamic.SetScalarParameterValue` _material_instance "Tex2_RotateAngle Z" (`self.Tex2_RotateAngle Z`))
  (`MaterialInstanceDynamic.SetScalarParameterValue` _returnvalue "Tex2_RotateAngle Y" (`self.Tex2_RotateAngle Y`))
  (`MaterialInstanceDynamic.SetScalarParameterValue` _material_instance "Tex2_RotateAngle Y" (`self.Tex2_RotateAngle Y`))
  (`MaterialInstanceDynamic.SetScalarParameterValue` _returnvalue "Tex2_Red_Level" (`self.Tex2_Red_Level`))
  (`MaterialInstanceDynamic.SetScalarParameterValue` _material_instance "Tex2_Red_Level" (`self.Tex2_Red_Level`))
  (`MaterialInstanceDynamic.SetScalarParameterValue` _returnvalue "Tex2_Green_Level" (`self.Tex2_Green_Level`))
  (`MaterialInstanceDynamic.SetScalarParameterValue` _material_instance "Tex2_Green_Level" (`self.Tex2_Green_Level`))
  (`MaterialInstanceDynamic.SetScalarParameterValue` _returnvalue "Tex2_Blue_Level" (`self.Tex2_Blue_Level`))
  (`MaterialInstanceDynamic.SetScalarParameterValue` _material_instance "Tex2_Blue_Level" (`self.Tex2_Blue_Level`))
  (`MaterialInstanceDynamic.SetScalarParameterValue` _returnvalue "Tex2_Power" (`self.Tex2_Power`))
  (`MaterialInstanceDynamic.SetScalarParameterValue` _material_instance "Tex2_Power" (`self.Tex2_Power`))
  (`MaterialInstanceDynamic.SetScalarParameterValue` _returnvalue "Tex2_Saturation" (`self.Tex2_Saturation`))
  (`MaterialInstanceDynamic.SetScalarParameterValue` _material_instance "Tex2_Saturation" (`self.Tex2_Saturation`))
  (`MaterialInstanceDynamic.SetScalarParameterValue` _returnvalue "Tex2_Tone" (`self.Tex2_Tone`))
  (`MaterialInstanceDynamic.SetScalarParameterValue` _material_instance "Tex2_Tone" (`self.Tex2_Tone`))
  (`MaterialInstanceDynamic.SetTextureParameterValue` _returnvalue "Tex3_Color" (`self.Tex3_Color`))
  (`MaterialInstanceDynamic.SetTextureParameterValue` _material_instance "Tex3_Color" (`self.Tex3_Color`))
  (`MaterialInstanceDynamic.SetVectorParameterValue` _returnvalue "Tex3_Scale" (`self.Tex3_Scale`))
  (`MaterialInstanceDynamic.SetVectorParameterValue` _material_instance "Tex3_Scale" (`self.Tex3_Scale`))
  (`MaterialInstanceDynamic.SetScalarParameterValue` _returnvalue "Tex3_Radius" (`self.Tex3_Radius`))
  (`MaterialInstanceDynamic.SetScalarParameterValue` _material_instance "Tex3_Radius" (`self.Tex3_Radius`))
  (`MaterialInstanceDynamic.SetScalarParameterValue` _returnvalue "Tex3_Density" (`self.Tex3_Density`))
  (`MaterialInstanceDynamic.SetScalarParameterValue` _material_instance "Tex3_Density" (`self.Tex3_Density`))
  (`MaterialInstanceDynamic.SetScalarParameterValue` _returnvalue "Tex3_RotateAngle Z" (`self.Tex3_RotateAngle Z`))
  (`MaterialInstanceDynamic.SetScalarParameterValue` _material_instance "Tex3_RotateAngle Z" (`self.Tex3_RotateAngle Z`))
  (`MaterialInstanceDynamic.SetScalarParameterValue` _returnvalue "Tex3_RotateAngle Y" (`self.Tex3_RotateAngle Y`))
  (`MaterialInstanceDynamic.SetScalarParameterValue` _material_instance "Tex3_RotateAngle Y" (`self.Tex3_RotateAngle Y`))
  (`MaterialInstanceDynamic.SetScalarParameterValue` _returnvalue "Tex3_Red_Level" (`self.Tex3_Red_Level`))
  (`MaterialInstanceDynamic.SetScalarParameterValue` _material_instance "Tex3_Red_Level" (`self.Tex3_Red_Level`))
  (`MaterialInstanceDynamic.SetScalarParameterValue` _returnvalue "Tex3_Green_Level" (`self.Tex3_Green_Level`))
  (`MaterialInstanceDynamic.SetScalarParameterValue` _material_instance "Tex3_Green_Level" (`self.Tex3_Green_Level`))
  (`MaterialInstanceDynamic.SetScalarParameterValue` _returnvalue "Tex3_Blue_Level" (`self.Tex3_Blue_Level`))
  (`MaterialInstanceDynamic.SetScalarParameterValue` _material_instance "Tex3_Blue_Level" (`self.Tex3_Blue_Level`))
  (`MaterialInstanceDynamic.SetScalarParameterValue` _returnvalue "Tex3_Power" (`self.Tex3_Power`))
  (`MaterialInstanceDynamic.SetScalarParameterValue` _material_instance "Tex3_Power" (`self.Tex3_Power`))
  (`MaterialInstanceDynamic.SetScalarParameterValue` _returnvalue "Tex3_Saturation" (`self.Tex3_Saturation`))
  (`MaterialInstanceDynamic.SetScalarParameterValue` _material_instance "Tex3_Saturation" (`self.Tex3_Saturation`))
  (`MaterialInstanceDynamic.SetScalarParameterValue` _returnvalue "Tex3_Tone" (`self.Tex3_Tone`))
  (`MaterialInstanceDynamic.SetScalarParameterValue` _material_instance "Tex3_Tone" (`self.Tex3_Tone`))
  (`MaterialInstanceDynamic.SetTextureParameterValue` _returnvalue "Tex4_Color" (`self.Tex4_Color`))
  (`MaterialInstanceDynamic.SetTextureParameterValue` _material_instance "Tex4_Color" (`self.Tex4_Color`))
  (`MaterialInstanceDynamic.SetVectorParameterValue` _returnvalue "Tex4_Scale" (`self.Tex4_Scale`))
  (`MaterialInstanceDynamic.SetVectorParameterValue` _material_instance "Tex4_Scale" (`self.Tex4_Scale`))
  (`MaterialInstanceDynamic.SetScalarParameterValue` _returnvalue "Tex4_Radius" (`self.Tex4_Radius`))
  (`MaterialInstanceDynamic.SetScalarParameterValue` _material_instance "Tex4_Radius" (`self.Tex4_Radius`))
  (`MaterialInstanceDynamic.SetScalarParameterValue` _returnvalue "Tex4_Density" (`self.Tex4_Density`))
  (`MaterialInstanceDynamic.SetScalarParameterValue` _material_instance "Tex4_Density" (`self.Tex4_Density`))
  (`MaterialInstanceDynamic.SetScalarParameterValue` _returnvalue "Tex4_RotateAngle Z" (`self.Tex4_RotateAngle Z`))
  (`MaterialInstanceDynamic.SetScalarParameterValue` _material_instance "Tex4_RotateAngle Z" (`self.Tex4_RotateAngle Z`))
  (`MaterialInstanceDynamic.SetScalarParameterValue` _returnvalue "Tex4_RotateAngle Y" (`self.Tex4_RotateAngle Y`))
  (`MaterialInstanceDynamic.SetScalarParameterValue` _material_instance "Tex4_RotateAngle Y" (`self.Tex4_RotateAngle Y`))
  (`MaterialInstanceDynamic.SetScalarParameterValue` _returnvalue "Tex4_Red_Level" (`self.Tex4_Red_Level`))
  (`MaterialInstanceDynamic.SetScalarParameterValue` _material_instance "Tex4_Red_Level" (`self.Tex4_Red_Level`))
  (`MaterialInstanceDynamic.SetScalarParameterValue` _returnvalue "Tex4_Green_Level" (`self.Tex4_Green_Level`))
  (`MaterialInstanceDynamic.SetScalarParameterValue` _material_instance "Tex4_Green_Level" (`self.Tex4_Green_Level`))
  (`MaterialInstanceDynamic.SetScalarParameterValue` _returnvalue "Tex4_Blue_Level" (`self.Tex4_Blue_Level`))
  (`MaterialInstanceDynamic.SetScalarParameterValue` _material_instance "Tex4_Blue_Level" (`self.Tex4_Blue_Level`))
  (`MaterialInstanceDynamic.SetScalarParameterValue` _returnvalue "Tex4_Power" (`self.Tex4_Power`))
  (`MaterialInstanceDynamic.SetScalarParameterValue` _material_instance "Tex4_Power" (`self.Tex4_Power`))
  (`MaterialInstanceDynamic.SetScalarParameterValue` _returnvalue "Tex4_Saturation" (`self.Tex4_Saturation`))
  (`MaterialInstanceDynamic.SetScalarParameterValue` _material_instance "Tex4_Saturation" (`self.Tex4_Saturation`))
  (`MaterialInstanceDynamic.SetScalarParameterValue` _returnvalue "Tex4_Tone" (`self.Tex4_Tone`))
  (`MaterialInstanceDynamic.SetScalarParameterValue` _material_instance "Tex4_Tone" (`self.Tex4_Tone`))
  (`MaterialInstanceDynamic.SetTextureParameterValue` _returnvalue "Tex5_Color" (`self.Tex5_Color`))
  (`MaterialInstanceDynamic.SetTextureParameterValue` _material_instance "Tex5_Color" (`self.Tex5_Color`))
  (`MaterialInstanceDynamic.SetVectorParameterValue` _returnvalue "Tex5_Scale" (`self.Tex5_Scale`))
  (`MaterialInstanceDynamic.SetVectorParameterValue` _material_instance "Tex5_Scale" (`self.Tex5_Scale`))
  (`MaterialInstanceDynamic.SetScalarParameterValue` _returnvalue "Tex5_Radius" (`self.Tex5_Radius`))
  (`MaterialInstanceDynamic.SetScalarParameterValue` _material_instance "Tex5_Radius" (`self.Tex5_Radius`))
  (`MaterialInstanceDynamic.SetScalarParameterValue` _returnvalue "Tex5_Density" (`self.Tex5_Density`))
  (`MaterialInstanceDynamic.SetScalarParameterValue` _material_instance "Tex5_Density" (`self.Tex5_Density`))
  (`MaterialInstanceDynamic.SetScalarParameterValue` _returnvalue "Tex5_RotateAngle Z" (`self.Tex5_RotateAngle Z`))
  (`MaterialInstanceDynamic.SetScalarParameterValue` _material_instance "Tex5_RotateAngle Z" (`self.Tex5_RotateAngle Z`))
  (`MaterialInstanceDynamic.SetScalarParameterValue` _returnvalue "Tex5_RotateAngle Y" (`self.Tex5_RotateAngle Y`))
  (`MaterialInstanceDynamic.SetScalarParameterValue` _material_instance "Tex5_RotateAngle Y" (`self.Tex5_RotateAngle Y`))
  (`MaterialInstanceDynamic.SetScalarParameterValue` _returnvalue "Tex5_Red_Level" (`self.Tex5_Red_Level`))
  (`MaterialInstanceDynamic.SetScalarParameterValue` _material_instance "Tex5_Red_Level" (`self.Tex5_Red_Level`))
  (`MaterialInstanceDynamic.SetScalarParameterValue` _returnvalue "Tex5_Green_Level" (`self.Tex5_Green_Level`))
  (`MaterialInstanceDynamic.SetScalarParameterValue` _material_instance "Tex5_Green_Level" (`self.Tex5_Green_Level`))
  (`MaterialInstanceDynamic.SetScalarParameterValue` _returnvalue "Tex5_Blue_Level" (`self.Tex5_Blue_Level`))
  (`MaterialInstanceDynamic.SetScalarParameterValue` _material_instance "Tex5_Blue_Level" (`self.Tex5_Blue_Level`))
  (`MaterialInstanceDynamic.SetScalarParameterValue` _returnvalue "Tex5_Power" (`self.Tex5_Power`))
  (`MaterialInstanceDynamic.SetScalarParameterValue` _material_instance "Tex5_Power" (`self.Tex5_Power`))
  (`MaterialInstanceDynamic.SetScalarParameterValue` _returnvalue "Tex5_Saturation" (`self.Tex5_Saturation`))
  (`MaterialInstanceDynamic.SetScalarParameterValue` _material_instance "Tex5_Saturation" (`self.Tex5_Saturation`))
  (`MaterialInstanceDynamic.SetScalarParameterValue` _returnvalue "Tex5_Tone" (`self.Tex5_Tone`))
  (`MaterialInstanceDynamic.SetScalarParameterValue` _material_instance "Tex5_Tone" (`self.Tex5_Tone`))
  (`MaterialInstanceDynamic.SetScalarParameterValue` _returnvalue "Emissive" (`self.Emissive`))
  (`MaterialInstanceDynamic.SetScalarParameterValue` _returnvalue "Opacity" (`self.Opacity`)))