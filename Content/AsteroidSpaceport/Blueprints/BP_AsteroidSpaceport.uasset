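; Asteroid spaceport prop with proximity-triggered animated doors and selectable color material.
; After a one-second startup gate, Tick checks camera distance to the bottom door, using paired DoOnce nodes to play or reverse the door timeline with open and close sounds.
; The construction script applies the color material and, when animation is disabled, poses the doors from DoorRotation.
; An optional demo loop cycles the colors every few seconds.
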(event `self.ReceiveTick`
  (params (DeltaSeconds :type "Float (single-precision)"))
  (`/Engine/EditorBlueprintResources/StandardMacros.Gate` true :!label _label
    (:`Exit`
      (if (`self.Animate`)
        (if (< (`KismetMathLibrary.VSize` (- (`PlayerCameraManager.GetCameraLocation` (`GameplayStatics.GetPlayerCameraManager` 0)) (`SceneComponent.K2_GetComponentLocation` (`self.SM_Spaceport_Door_Bot`)))) (`self.Animation_Trigger_Distance`))
          (`|ExecutionSequence`
            (:`then_0`
              (`/Engine/EditorBlueprintResources/StandardMacros.DoOnce` false :!label _label_2
                (:`Completed`
                  (set `self.FirstTime` false)
                  (`AudioComponent.Play` (`self.SC_Scifi_Door_Open`) 0.0)
                  (bind (_direction _doors) (`Timeline|Door_Anim` :!label _label_3)
                    (:`Update`
                      (set `self.Door Rotation` _doors)
                      (`self.Update_Doors`))))))
            (:`then_1`
              (goto _label_4 :!via `Reset`))
            (:`then_2`
              (`AudioComponent.Stop` (`self.SC_Scifi_Door_Close`))))
          (elif (not (`self.FirstTime`))
            (`|ExecutionSequence`
              (:`then_0`
                (`/Engine/EditorBlueprintResources/StandardMacros.DoOnce` false :!label _label_4
                  (:`Completed`
                    (`AudioComponent.Play` (`self.SC_Scifi_Door_Close`) 0.0)
                    (goto _label_3 :!via `Reverse`))))
              (:`then_1`
                (goto _label_2 :!via `Reset`))
              (:`then_2`
                (`AudioComponent.Stop` (`self.SC_Scifi_Door_Open`))))))))))

(event `self.ReceiveBeginPlay`
  (bind _color (`self.Color`))
  (`|ExecutionSequence`
    (:`then_0`
      (`KismetSystemLibrary.Delay` 1.0)
      (goto _label :!via `Open`))
    (:`then_1`
      (if (`self.Color Change Demo`)
        (`KismetSystemLibrary.Delay` 3.0 :!label _label_5)
        (if (== _color 4)
          (set `self.Color` 0)
          (else
            (set `self.Color` (+ _color 1))))
        (`self.Select Material from Color Variable`)
        (`self.Set Material to Meshes`)
        (goto _label_5)))))

(fn `Select Material from Color Variable`
  (switch `int` (`self.Color`)
    (:`0`
      (set `self.Material` "/Game/AsteroidSpaceport/Materials/Stations/MI_Spaceport_Red.MI_Spaceport_Red"))
    (:`1`
      (set `self.Material` "/Game/AsteroidSpaceport/Materials/Stations/MI_Spaceport_Blue.MI_Spaceport_Blue"))
    (:`2`
      (set `self.Material` "/Game/AsteroidSpaceport/Materials/Stations/MI_Spaceport_Yellow.MI_Spaceport_Yellow"))
    (:`3`
      (set `self.Material` "/Game/AsteroidSpaceport/Materials/Stations/MI_Spaceport_Grey.MI_Spaceport_Grey"))
    (:`4`
      (set `self.Material` "/Game/AsteroidSpaceport/Materials/Stations/MI_Spaceport.MI_Spaceport"))))

(fn `Set Material to Meshes`
  (`PrimitiveComponent.SetMaterial` (`self.Interior`) 0 (`self.Material`))
  (`PrimitiveComponent.SetMaterial` (`self.Spaceport`) 0 (`self.Material`))
  (`PrimitiveComponent.SetMaterial` (`self.SM_Spaceport_Door_Top`) 0 (`self.Material`))
  (`PrimitiveComponent.SetMaterial` (`self.SM_Spaceport_Door_Bot`) 0 (`self.Material`)))

(fn `Update_Doors`
  (`SceneComponent.K2_SetRelativeRotation` (`self.SM_Spaceport_Door_Bot`) (`KismetMathLibrary.MakeRotator` (`KismetMathLibrary.Lerp` 0.0 100.0 (`self.Door Rotation`))) false false)
  (`SceneComponent.K2_SetRelativeRotation` (`self.SM_Spaceport_Door_Top`) (`KismetMathLibrary.MakeRotator` (`KismetMathLibrary.Lerp` 0.0 -100.0 (`self.Door Rotation`))) false false))

(fn `UserConstructionScript`
  (`self.Select Material from Color Variable`)
  (`self.Set Material to Meshes`)
  (if (not (`self.Animate`))
    (`self.Update_Doors`)))