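; Asteroid Blueprint for the spaceport that randomizes its mesh and orientation in the construction script.
; A random integer type selects the small asteroid mesh in one of three cases and the medium mesh otherwise.
; The script then stores the mesh's world scale and applies a random world rotation including roll.
; The event graph holds no active logic.
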(fn `UserConstructionScript`
  (bind _staticmesh (`self.StaticMesh`))
  (bind _output_get (set `self.AsteroidType` (`KismetMathLibrary.RandomIntegerInRange` 0 2)))
  (switch `int` _output_get
    (:`Default`
      (`StaticMeshComponent.SetStaticMesh` _staticmesh "/Game/AsteroidSpaceport/Meshes/Asteroids/SM_Spaceport_Asteroid_Medium.SM_Spaceport_Asteroid_Medium" :!label _label))
    (:`0`
      (goto _label))
    (:`1`
      (`StaticMeshComponent.SetStaticMesh` _staticmesh "/Game/AsteroidSpaceport/Meshes/Asteroids/SM_Spaceport_Asteroid_Small.SM_Spaceport_Asteroid_Small")))
  (set `self.Scale` (`SceneComponent.K2_GetComponentScale` (`self.StaticMesh`)))
  (`SceneComponent.K2_SetWorldRotation` (`self.StaticMesh`) (`KismetMathLibrary.RandomRotator` true) false false))