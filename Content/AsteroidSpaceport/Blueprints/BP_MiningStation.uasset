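; BP_MiningStation is a modular space mining station prop with animated parts and a selectable color scheme.
; Tick slowly spins the ring, entry signboard and two asteroids at fixed per-frame rates, not scaled by delta time.
; The construction script maps the Color variable to a material instance and applies it to the main station meshes.
; An optional ColorChangeDemo flag starts a BeginPlay delay loop that cycles through the colors.
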(event `self.ReceiveTick`
  (params (DeltaSeconds :type "Float (single-precision)"))
  (`SceneComponent.K2_AddLocalRotation` (`self.SM_Mining_Ring`) (struct :`Yaw` 0.1) false false)
  (`SceneComponent.K2_AddLocalRotation` (`self.SM_Mining_Entry_Signboard`) (struct :`Yaw` -0.1) false false)
  (`SceneComponent.K2_AddLocalRotation` (`self.SM_Mining_Asteroid_Large`) (struct :`Yaw` -0.01) false false)
  (`SceneComponent.K2_AddLocalRotation` (`self.SM_Mining_Asteroid_Med`) (struct :`Yaw` 0.01) false false))

(event `self.ReceiveBeginPlay`
  (bind _color (`self.Color`))
  (if (`self.Color Change Demo`)
    (`KismetSystemLibrary.Delay` 3.0 :!label _label)
    (if (== _color 4)
      (set `self.Color` 0)
      (else
        (set `self.Color` (+ _color 1))))
    (`self.Select Material from Color Variable`)
    (`self.Set Material to Meshes`)
    (goto _label)))

(fn `Select Material from Color Variable`
  (switch `int` (`self.Color`)
    (:`0`
      (set `self.Material` "/Game/AsteroidSpaceport/Materials/Stations/MI_ModularMiningStation_Red.MI_ModularMiningStation_Red"))
    (:`1`
      (set `self.Material` "/Game/AsteroidSpaceport/Materials/Stations/MI_ModularMiningStation_Blue.MI_ModularMiningStation_Blue"))
    (:`2`
      (set `self.Material` "/Game/AsteroidSpaceport/Materials/Stations/MI_ModularMiningStation_Yellow.MI_ModularMiningStation_Yellow"))
    (:`3`
      (set `self.Material` "/Game/AsteroidSpaceport/Materials/Stations/MI_ModularMiningStation_Grey.MI_ModularMiningStation_Grey"))
    (:`4`
      (set `self.Material` "/Game/AsteroidSpaceport/Materials/Stations/MI_ModularMiningStation.MI_ModularMiningStation"))))

(fn `Set Material to Meshes`
  (`PrimitiveComponent.SetMaterial` (`self.SM_Mining_Entry`) 0 (`self.Material`))
  (`PrimitiveComponent.SetMaterial` (`self.SM_Mining_Ring`) 0 (`self.Material`))
  (`PrimitiveComponent.SetMaterial` (`self.SM_Mining_Torus`) 0 (`self.Material`))
  (`PrimitiveComponent.SetMaterial` (`self.SM_Mining_Tower`) 0 (`self.Material`))
  (`PrimitiveComponent.SetMaterial` (`self.SM_Mining_Ring_Small`) 0 (`self.Material`)))

(fn `UserConstructionScript`
  (`self.Select Material from Color Variable`)
  (`self.Set Material to Meshes`))